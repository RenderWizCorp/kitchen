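; BP_TLOM_Fridge_01 is a fridge prop whose two doors and five drawers are posed by variables in the Construction Script.
; WingTop and WingBottom set the yaw of the top and bottom door meshes.
; Separate variables slide the B drawer, glass drawer and three freezer drawers along local Y, as offsets added to their current transforms.
; The script contains only this static posing, with no interaction or animation logic.
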(fn ConstructionScript
  (Transformation|SetRelativeRotation (Variables|Default|GetSM_TLOM_Fridge_01_Wing_Top) (Math|Rotator|MakeRotator 0.0 0.0 (Variables|Default|GetWing_Top)) false false)
  (Transformation|SetRelativeRotation (Variables|Default|GetSM_TLOM_Fridge_01_Wing_Bottom) (Math|Rotator|MakeRotator 0.0 0.0 (Variables|Default|GetWing_Bottom)) false false)
  (Class|SceneComponent|AddLocalTransform (Variables|Default|GetSM_TLOM_Fridge_01_Drawer_B) (Math|Conversions|ToTransform(Vector) (Math|Vector|MakeVector 0.0 (Variables|Default|GetDrawer_B) 0.0)) false false)
  (Class|SceneComponent|AddLocalTransform (Variables|Default|GetSM_TLOM_Fridge_01_Drawer_WithGlass) (Math|Conversions|ToTransform(Vector) (Math|Vector|MakeVector 0.0 (Variables|Default|GetDrawer_Glass) 0.0)) false false)
  (Class|SceneComponent|AddLocalTransform (Variables|Default|GetSM_TLOM_Fridge_01_Drawer_Freezer) (Math|Conversions|ToTransform(Vector) (Math|Vector|MakeVector 0.0 (Variables|Default|GetDrawer_Freezer_1) 0.0)) false false)
  (Class|SceneComponent|AddLocalTransform (Variables|Default|GetSM_TLOM_Fridge_01_Drawer_Freezer1) (Math|Conversions|ToTransform(Vector) (Math|Vector|MakeVector 0.0 (Variables|Default|GetDrawer_Freezer_2) 0.0)) false false)
  (Class|SceneComponent|AddLocalTransform (Variables|Default|GetSM_TLOM_Fridge_01_Drawer_Freezer2) (Math|Conversions|ToTransform(Vector) (Math|Vector|MakeVector 0.0 (Variables|Default|GetDrawer_Freezer_3) 0.0)) false false))