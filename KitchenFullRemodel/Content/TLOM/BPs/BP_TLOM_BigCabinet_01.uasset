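; Prop Blueprint for a big cabinet with a rotatable wing and three drawers, posed through variables.
; The construction script sets the wing's relative yaw from the Wing variable and shifts each drawer along its local Y axis by its own offset variable.
; Drawer offsets are added to each component's existing transform, while the wing rotation is set outright.
; The file shows no runtime logic.
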(fn ConstructionScript
  (Transformation|SetRelativeRotation (Variables|Default|GetSM_TLOM_BigCabinet_01_Wing) (Math|Rotator|MakeRotator 0.0 0.0 (Variables|Default|GetWing)) false false)
  (Class|SceneComponent|AddLocalTransform (Variables|Default|GetSM_TLOM_BigCabinet_01_Drawer) (Math|Conversions|ToTransform(Vector) (Math|Vector|MakeVector 0.0 (Variables|Default|GetDrawer_0) 0.0)) false false)
  (Class|SceneComponent|AddLocalTransform (Variables|Default|GetSM_TLOM_BigCabinet_01_Drawer1) (Math|Conversions|ToTransform(Vector) (Math|Vector|MakeVector 0.0 (Variables|Default|GetDrawer_1) 0.0)) false false)
  (Class|SceneComponent|AddLocalTransform (Variables|Default|GetSM_TLOM_BigCabinet_01_Drawer2) (Math|Conversions|ToTransform(Vector) (Math|Vector|MakeVector 0.0 (Variables|Default|GetDrawer_2) 0.0)) false false))