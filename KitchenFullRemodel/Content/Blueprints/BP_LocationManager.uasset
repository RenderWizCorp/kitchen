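; BP_LocationManager cycles the player through viewpoints by possessing each BP_LookAround actor found in the level.
; On BeginPlay it gathers those actors, possesses the first, creates the BP_Interface widget and registers the input mapping context.
; A completed IA_Click possesses the next point, wrapping at the end, with a DoOnce and delay acting as a cooldown.
; The first click also fades out the interface.
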(event Custom|MovePoint
  (bind _allpoints (Variables|Default|GetAllPoints))
  (if (> (+ (Variables|Default|GetCurrentIndex) 1) (Utilities|Array|Length _allpoints))
    (Variables|Default|SetCurrentIndex 0))
  (Default|Possess (Utilities|Array|Get(acopy) _allpoints (Variables|Default|GetCurrentIndex)))
  (Math|Integer|IncrementInt (Variables|Default|GetCurrentIndex)))

(event Input|EnhancedActionEvents|EnhancedInputActionIA_Click
  (params (ActionValue :type Boolean) (ElapsedSeconds :type Float%20%28double-precision%29) (TriggeredSeconds :type Float%20%28double-precision%29) (InputAction :type Input%20Action%20Object%20Reference :default "/Game/Blueprints/Backend/IA_Click.IA_Click"))
  (bind _allpoints (Variables|Default|GetAllPoints))
  (Utilities|FlowControl|DoOnce false :!label _label
    (:Completed
      (Utilities|FlowControl|Sequence
        (:then_0
          (if (> (+ (Variables|Default|GetCurrentIndex) 1) (Utilities|Array|Length _allpoints))
            (Variables|Default|SetCurrentIndex 0))
          (Default|Possess (Utilities|Array|Get(acopy) _allpoints (Variables|Default|GetCurrentIndex)))
          (Math|Integer|IncrementInt (Variables|Default|GetCurrentIndex)))
        (:then_1
          (Utilities|FlowControl|DoOnce false
            (:Completed
              (Default|FadeOut (Variables|Default|GetInterfaceWidget)))))
        (:then_2
          (Utilities|FlowControl|Delay 2.0)
          (goto _label Reset))))))

(event EventBeginPlay
  (bind _returnvalue (Game|GetPlayerController 0))
  (bind _returnvalue_2 (PlayerController|LocalPlayerSubsystems|GetEnhancedInputLocalPlayerSubsystem _returnvalue))
  (bind _outactors (Actor|GetAllActorsOfClass "/Game/Blueprints/BP_LookAround.BP_LookAround_C"))
  (Variables|Default|SetAllPoints _outactors)
  (CallFunction|MovePoint)
  (bind _returnvalue_3 (UserInterface|CreateWidget "/Game/Blueprints/Backend/BP_Interface.BP_Interface_C"))
  (bind _output_get (Variables|Default|SetInterfaceWidget _returnvalue_3))
  (UserInterface|Viewport|AddtoViewport _output_get 0)
  ;[1 1 1] input mapping
  (Utilities|IsValid _returnvalue_2
    (:Is%20Valid
      (Input|AddMappingContext _returnvalue_2 "/Game/Blueprints/Backend/IM_Inputs.IM_Inputs" 1 "(bIgnoreAllPressedKeysUntilRelease=True,bForceImmediately=False,bNotifyUserSettings=False)")
      (Input|SetInputModeGameOnly (Game|GetPlayerController 0) false))))

(event Collision|EventActorBeginOverlap
  (params (OtherActor :type Actor%20Object%20Reference)))

(event EventTick
  (params (DeltaSeconds :type Float%20%28single-precision%29)))

(fn ConstructionScript)