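; Pawn for a look-around view, steered in yaw and pitch by the IA_LookAround Enhanced Input action.
; Its Possess event makes player controller 0 possess it and adds the IM_Inputs mapping context.
; If the input subsystem is valid, it also clamps the camera manager's view using Pitch and Yaw ranges, with yaw limits offset from the current control rotation.
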(event Custom|Possess
  (bind _returnvalue (Game|GetPlayerController 0))
  (bind _returnvalue_2 (Game|GetPlayerCameraManager 0))
  (bind _returnvalue_3 (Pawn|GetControlRotation :!class /Script/Engine.Pawn))
  (bind _pitch (Variables|Default|GetPitch))
  (bind _yaw (Variables|Default|GetYaw))
  (bind (_min _max) (Utilities|Struct|BreakSTR_MinMax _yaw))
  (bind (_min_2 _max_2) (Utilities|Struct|BreakSTR_MinMax _pitch))
  (bind _returnvalue_4 (PlayerController|LocalPlayerSubsystems|GetEnhancedInputLocalPlayerSubsystem _returnvalue))
  (Pawn|Possess _returnvalue self)
  ;[1 1 1] input mapping
  (Utilities|IsValid _returnvalue_4
    (:Is%20Valid
      (Input|AddMappingContext _returnvalue_4 "/Game/Blueprints/Backend/IM_Inputs.IM_Inputs" 1 "(bIgnoreAllPressedKeysUntilRelease=True,bForceImmediately=False,bNotifyUserSettings=False)")
      ;[1 1 1] contraints
      ;;[1 1 1] up and down
      (Variables|/Script/Engine.PlayerCameraManager|SetViewPitchMin _returnvalue_2 _min_2)
      (Variables|/Script/Engine.PlayerCameraManager|SetViewPitchMax _returnvalue_2 _max_2)
      ;;[1 1 1] left right
      (Variables|/Script/Engine.PlayerCameraManager|SetViewYawMin _returnvalue_2 (+ (.yaw _returnvalue_3) _max))
      (Variables|/Script/Engine.PlayerCameraManager|SetViewYawMax _returnvalue_2 (- (.yaw _returnvalue_3) _min)))))

(event Input|EnhancedActionEvents|EnhancedInputActionIA_LookAround
  (params (ActionValue :type Vector%202D%20Structure) (ElapsedSeconds :type Float%20%28double-precision%29) (TriggeredSeconds :type Float%20%28double-precision%29) (InputAction :type Input%20Action%20Object%20Reference :default "/Game/Blueprints/Backend/IA_LookAround.IA_LookAround"))
  ;[1 1 1] Look Around Action
  ;;[1 1 1] left and right
  (Pawn|Input|AddControllerYawInput (.x ActionValue))
  ;;[1 1 1] up and down
  (Pawn|Input|AddControllerPitchInput (.y ActionValue)))

(event EventBeginPlay)

(event Collision|EventActorBeginOverlap
  (params (OtherActor :type Actor%20Object%20Reference)))

(event EventTick
  (params (DeltaSeconds :type Float%20%28single-precision%29)))

(fn ConstructionScript)