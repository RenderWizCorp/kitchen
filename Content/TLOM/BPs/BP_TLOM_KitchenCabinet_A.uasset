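; BP_TLOM_KitchenCabinet_A is a modular kitchen cabinet prop whose drawer and two wing doors can be posed.
; Its construction script offsets the drawer mesh along local Y by the Drawer value and yaws each door to its own WingA or WingB angle.
; The file shows no runtime logic, so the pose is set only at construction.
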(fn ConstructionScript
  (Class|SceneComponent|AddLocalTransform (Variables|Default|GetSM_TLOM_ModularCabinetParts_01_Drawer) (Math|Conversions|ToTransform(Vector) (Math|Vector|MakeVector 0.0 (Variables|Default|GetDrawer) 0.0)) false false)
  (Transformation|SetRelativeRotation (Variables|Default|GetSM_TLOM_ModularCabinetParts_01_Wing_D1) (Math|Rotator|MakeRotator 0.0 0.0 (Variables|Default|GetWing_A)) false false)
  (Transformation|SetRelativeRotation (Variables|Default|GetSM_TLOM_ModularCabinetParts_01_Wing_D) (Math|Rotator|MakeRotator 0.0 0.0 (Variables|Default|GetWing_B)) false false))