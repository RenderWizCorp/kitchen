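; BP_TLOM_OvenHub_01 is an oven hub prop whose wing and buttons can be posed through variables.
; The construction script sets the wing mesh's relative roll from the Wing value.
; It also sets the relative pitch of four A-type buttons, one B and one C, each from its own Button value.
; The file shows no runtime logic, so the pose is applied only at construction.
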(fn ConstructionScript
  (Transformation|SetRelativeRotation (Variables|Default|GetSM_TLOM_OvenHub_01_Wing) (Math|Rotator|MakeRotator (Variables|Default|GetWing) 0.0 0.0) false false)
  (Transformation|SetRelativeRotation (Variables|Default|GetSM_TLOM_OvenHub_01_Button_A) (Math|Rotator|MakeRotator 0.0 (Variables|Default|GetButton_0) 0.0) false false)
  (Transformation|SetRelativeRotation (Variables|Default|GetSM_TLOM_OvenHub_01_Button_A1) (Math|Rotator|MakeRotator 0.0 (Variables|Default|GetButton_1) 0.0) false false)
  (Transformation|SetRelativeRotation (Variables|Default|GetSM_TLOM_OvenHub_01_Button_A2) (Math|Rotator|MakeRotator 0.0 (Variables|Default|GetButton_2) 0.0) false false)
  (Transformation|SetRelativeRotation (Variables|Default|GetSM_TLOM_OvenHub_01_Button_A3) (Math|Rotator|MakeRotator 0.0 (Variables|Default|GetButton_3) 0.0) false false)
  (Transformation|SetRelativeRotation (Variables|Default|GetSM_TLOM_OvenHub_01_Button_B) (Math|Rotator|MakeRotator 0.0 (Variables|Default|GetButton_4) 0.0) false false)
  (Transformation|SetRelativeRotation (Variables|Default|GetSM_TLOM_OvenHub_01_Button_C) (Math|Rotator|MakeRotator 0.0 (Variables|Default|GetButton_5) 0.0) false false))